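; Component that mirrors a MetaSound output parameter back to an OSC client, as feedback for OSC audio control.
; OutputWatchStart watches the named output immediately for auto-activating audio components, otherwise once playback reports Playing.
; Float changes are normalized from the parameter range and sent to the given address.
; The raw value also goes out as a string to a WheelVal address built from that address's suffix.
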(event `OutputWatchStart`
  (params (AudComp :type "AudioComponent Object Reference") (OscAudioInformation :type "OscAudioControlAudioSpawn Structure (by ref)") (Client :type "OSCClient Object Reference") (Address :type String))
  ;[0 0 0] create event for when the audio playback starts for this audio comp, and then watch the metasound output
  (set `self.Address` Address)
  (set `self.Client` Client)
  (bind _output_get (set `self.AudComp` AudComp))
  (if (`ActorComponent.bAutoActivate` _output_get)
    (`MetaSoundOutputSubsystem.WatchOutput` (subsystem `MetaSoundOutputSubsystem`) (`self.AudComp`) (`.SoundParameterName` (break `OscAudioControlAudioSpawn` OscAudioInformation)) (`|CreateDelegate` :!event `AudComp1Watch`) "None" "None" :!label _label)
    (else
      (add `AudioComponent.OnAudioPlayStateChanged` _output_get (delegate `AudCompPlaybackStart`)))))

(event `AudCompPlaybackStart`
  (params (PlayState :type "EAudioComponentPlayState Enum" :default "Playing"))
  ;[0 0 0] create event for when the audio playback starts for this audio comp, and then watch the metasound output
  (switch `EAudioComponentPlayState` PlayState
    (:`Playing`
      (goto _label))))

(event `AudComp1Watch`
  (params (OutputName :type Name) (Output :type "MetaSoundOutput Structure (by ref)"))
  (bind _address (`self.Address`))
  ;[0 0 0] create event for when the audio playback starts for this audio comp, and then watch the metasound output
  (bind (_success _returnvalue) (`MetasoundOutputBlueprintAccess.GetFloat` Output))
  (if _success
    (bind (_x _y) (`KismetMathLibrary.BreakVector2D` (`.ParameterRange` (break `OscAudioControlAudioSpawn` (stale `OutputWatchStart` OscAudioInformation)))))
    (`/OscAudioControl/BPL_OscAudioControlHelpers.OscSendFloat` _address (`KismetMathLibrary.MapRangeClamped` _returnvalue _x _y 0.0 1.0) (`self.Client`))
    (`/OscAudioControl/BPL_OscAudioControlHelpers.OscSendString` (`KismetStringLibrary.Concat_StrStr` "/4/WheelVal" (`.RightS` (`KismetStringLibrary.Split` _address "-"))) (`KismetStringLibrary.Conv_DoubleToString` _returnvalue) (`self.Client`))))